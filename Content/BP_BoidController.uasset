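; Boid flocking controller Blueprint holding debug and visualization helpers for BoidDatas; the flocking math is not in these graphs.
; Helper functions draw one boid's radii, vectors and vision cone, trail a camera behind the first boid, and project a lockable mouse seek target.
; Only cursor display and an empty Tick loop are live.
; Niagara, particle and instanced-mesh rendering experiments, helper calls and target controls are all disconnected.
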(event EventTick
  (params (DeltaSeconds :type Float%20%28single-precision%29))
  (for _array_element (Variables|Default|GetBoidDatas)
    _))

(event EventBeginPlay
  (Variables|/Script/Engine.PlayerController|SetbShowMouseCursor (Game|GetPlayerController 0) true))

(event Input|MouseEvents|MouseWheelUp
  (params (Key :type Key%20Structure :default "None")))

(event Input|MouseEvents|MouseWheelDown
  (params (Key :type Key%20Structure :default "None")))

(event Input|MouseEvents|LeftMouseButton
  (params (Key :type Key%20Structure :default "None")))

(fn ConstructionScript)

(fn ShowBoidDebugVisuals
  (params (Boid :type Boid%20Data%20Structure%20%28by%20ref%29))
  (bind _returnvalue (Math|Vector|Normalize (.velocity Boid)))
  (bind _linemultiplier (LocalVariables|GetLineMultiplier))
  (bind _visionconeangle (Variables|Default|GetVisionConeAngle))
  (bind _returnvalue_2 (/ _visionconeangle 2.0))
  (Rendering|Debug|DrawDebugSphere (.location (.transform Boid)) (Variables|Default|GetSeperationRadius) 20 "(R=1.000000,G=0.226567,B=0.813674,A=0.500000)" 0.0 (/ (LocalVariables|GetLineThickness) 2.0))
  (Rendering|Debug|DrawDebugLine (.location (.transform Boid)) (+ (.location (.transform Boid)) (* _returnvalue _linemultiplier)) "(R=0.020223,G=1.000000,B=0.000000,A=1.000000)" 0.0 (LocalVariables|GetLineThickness))
  (Rendering|Debug|DrawDebugLine (.location (.transform Boid)) (+ (.location (.transform Boid)) (* (Math|Vector|Normalize (.acceleration Boid)) _linemultiplier)) "(R=0.000000,G=0.129302,B=1.000000,A=1.000000)" 0.0 (LocalVariables|GetLineThickness))
  (Class|KismetSystemLibrary|DrawDebugConeinDegrees (.location (.transform Boid)) _returnvalue (Variables|Default|GetNeighbourRadius) _returnvalue_2 _returnvalue_2 18 "(R=0.005214,G=0.000000,B=1.000000,A=1.000000)" 0.0 (/ (LocalVariables|GetLineThickness) 2.0))
  (Rendering|Debug|DrawDebugPoint (.location (.transform Boid)) 1e+01 "(R=0.000000,G=0.137149,B=0.843750,A=1.000000)" 1.0))

(fn DrawDebug
  (if (Variables|Default|GetbShowDebug)
    (CallFunction|ShowBoidDebugVisuals (Utilities|Array|Get(acopy) (Variables|Default|GetBoidDatas) (Variables|Default|GetDebugIndex)))))

(fn UpdateCamera
  (bind _boiddatas (Variables|Default|GetBoidDatas))
  (bind _output (Utilities|Array|Get(acopy) _boiddatas))
  (Transformation|SetActorTransform (Variables|Default|GetDebugCamera) (Math|Transform|MakeTransform (- (.location (.transform _output)) (* (+ (Math|Vector|Normalize (.velocity _output)) "0,0.500000, 0") 4e+02)) (Math|Rotator|MakeRotfromX (.velocity _output)))))

(fn SpawnDebugCamera
  (bind _returnvalue (Game|SpawnActorfromClass "/Script/Engine.CameraActor" (Math|Transform|MakeTransform "0, 0, 0") "Undefined" 0 0))
  (bind _output_get (Variables|Default|SetDebugCamera _returnvalue))
  (Class|CameraComponent|SetConstraintAspectRatio (Variables|/Script/Engine.CameraActor|GetCameraComponent _output_get) false))

(fn MouseTest
  (bind _returnvalue (Game|GetPlayerController 0))
  (bind (_worldlocation _worlddirection) (Game|Player|ConvertMouseLocationToWorldSpace _returnvalue))
  (Rendering|Debug|DrawDebugSphere (.location (Variables|Default|GetSeekTransform)) 5e+01 8 "(R=1.000000,G=0.014252,B=0.000000,A=1.000000)" 0.0 3e+01)
  (if (not (Variables|Default|GetLockMouseTarget))
    (Variables|Default|SetSeekTransform (Math|Transform|MakeTransform (+ _worldlocation (* _worlddirection (Variables|Default|GetMousePointerDistance)))))))